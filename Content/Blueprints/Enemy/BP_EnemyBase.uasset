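; BP_EnemyBase is a base enemy Blueprint that provides dissolve effects for the enemy and its weapon.
; Two events each receive a dynamic material instance and play their own timeline, writing its curve into the "Dissolve" scalar parameter every update.
; Disconnected highlight leftovers (debug sphere, custom depth toggles) never run, and Tick and the construction script are empty.
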(event `self.ReceiveTick`
  (params (DeltaSeconds :type "Float (single-precision)")))

(event `self.StartDissolveTimeline`
  (params (DynamicMaterialInstance :type "MaterialInstanceDynamic Object Reference"))
  (bind (_direction `_新建轨道_0`) (`Timeline|溶解时间轴`)
    (:`Update`
      (`MaterialInstanceDynamic.SetScalarParameterValue` DynamicMaterialInstance "Dissolve" `_新建轨道_0`))))

(event `self.StartWeaponDissolveTimeline`
  (params (DynamicMaterialInstance :type "MaterialInstanceDynamic Object Reference"))
  (bind (_direction `_新建轨道_0`) (`Timeline|时间轴`)
    (:`Update`
      (`MaterialInstanceDynamic.SetScalarParameterValue` DynamicMaterialInstance "Dissolve" `_新建轨道_0`))))

(fn `UserConstructionScript`)